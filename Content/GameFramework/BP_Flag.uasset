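; BP_Flag is a team flag actor that can be moved, hidden and returned to where it started.
; On BeginPlay it caches its starting transform and applies a red or blue material to its static mesh based on IsTeamA.
; Its events teleport it back to that transform, move it to a given location, or toggle mesh visibility and collision together.
; It has no overlap or tick logic of its own.
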(event Custom|ReturnFlag
  (Transformation|SetActorTransform (Variables|Default|GetInitialTransform) false true))

(event Custom|EnableFlag
  (params (IsEnabled :type Boolean))
  (Rendering|SetVisibility (Variables|Debug|GetStaticMeshComponent) IsEnabled false)
  (if IsEnabled
    (Collision|SetCollisionEnabled (Variables|Debug|GetStaticMeshComponent) "QueryAndPhysics")
    (else
      (Collision|SetCollisionEnabled (Variables|Debug|GetStaticMeshComponent) "NoCollision"))))

(event Custom|MoveToLocation
  (params (Location :type Vector))
  (Transformation|SetActorLocation Location false false))

(event EventBeginPlay
  (Variables|Default|SetInitialTransform (Transformation|GetActorTransform))
  (if (Variables|Default|GetIsTeamA)
    (Rendering|Material|SetMaterial (Variables|Debug|GetStaticMeshComponent) 0 "/Game/MapAssets/Materials/RedFlag.RedFlag")
    (else
      (Rendering|Material|SetMaterial (Variables|Debug|GetStaticMeshComponent) 0 "/Game/MapAssets/Materials/BlueFlag.BlueFlag"))))

(event Collision|EventActorBeginOverlap
  (params (OtherActor :type Actor%20Object%20Reference)))

(event EventTick
  (params (DeltaSeconds :type Float%20%28single-precision%29)))

(fn ConstructionScript)