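; Game mode that runs Capture the Flag matches: match start, flag pickup and drop, and base scoring.
; A ready counter triggers match start, then team assignment and the timer on CTF_GameState.
; Team checks on CTF_PlayerState return own flags or attach enemy flags to the player, and death drops them.
; Home-base scoring checks other characters for held flags inside a per-character loop, then resets the flag and increments the team score.
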(event Custom|StartCaptureTheFlag
  ;[1 1 1] Match Setup
  (Development|PrintString "Match Started!")
  (bind _asctf_game_state (Utilities|Casting|CastToCTF_GameState (Game|GetGameState)))
  (Default|AssignTeamsStates _asctf_game_state)
  (Default|StartTimer _asctf_game_state))

(event Custom|PlayerReady
  ;[1 1 1] Match Setup
  (bind _result (Math|Integer|IncrementInt (Variables|Default|GetReadyInstanceNum))
    (:%20%20
      (if (== _result 3)
        (Class|GameMode|StartMatch)
        (Utilities|FlowControl|Delay 0.0)
        (CallFunction|StartCapturetheFlag)))))

(event Custom|PlayerFlagEvent
  (params (Player :type BP%20Character%20Object%20Reference) (Flag :type BP%20Flag%20Object%20Reference))
  ;[1 1 1] Flag Logic
  (bind _asctf_player_state (Utilities|Casting|CastToCTF_PlayerState (Variables|/Script/Engine.Pawn|GetPlayerState Player)))
  (if (Math|Boolean|Equal(Boolean) (Variables|/Game/GameFramework/CTF_PlayerState.CTF_PlayerState_C|GetIsTeamA _asctf_player_state) (Variables|/Game/GameFramework/BP_Flag.BP_Flag_C|GetIsTeamA Flag))
    (Development|PrintString "Caught Own Flag")
    (Default|ReturnFlag Flag)
    (else
      (Development|PrintString "Caught Enemy Flag")
      (Default|SetFlag Player Flag)
      (Default|EnableFlag Flag false))))

(event Custom|Player%20Death
  (params (Player :type BP%20Character%20Object%20Reference))
  (bind _heldflag (Variables|/Game/GameFramework/BP_Character.BP_Character_C|GetHeldFlag Player))
  ;[1 1 1] Flag Logic
  (Default|EnableFlag _heldflag true)
  (Default|MovetoLocation _heldflag (+ (Transformation|GetActorLocation Player) "100.000000,100.000000, 0"))
  (Default|SetFlag Player))

(event Custom|PlayerBaseEvent
  (params (Player :type BP%20Character%20Object%20Reference) (Base :type BP%20Base%20Object%20Reference))
  (bind _heldflag (Variables|/Game/GameFramework/BP_Character.BP_Character_C|GetHeldFlag Player))
  ;[1 1 1] Base Logic
  (bind _asctf_player_state (Utilities|Casting|CastToCTF_PlayerState (Variables|/Script/Engine.Pawn|GetPlayerState Player)))
  (if (Math|Boolean|Equal(Boolean) (Variables|/Game/GameFramework/CTF_PlayerState.CTF_PlayerState_C|GetIsTeamA _asctf_player_state) (Variables|/Game/GameFramework/BP_Base.BP_Base_C|GetIsTeamA Base))
    (Development|PrintString "Home base")
    (Utilities|IsValid _heldflag
      (:Is%20Valid
        (Development|PrintString "Hello")
        (bind _outactors (Actor|GetAllActorsOfClass "/Game/GameFramework/BP_Character.BP_Character_C"))
        (for _array_element _outactors
          (if (!= _array_element Player)
            (Utilities|IsValid (Variables|/Game/GameFramework/BP_Character.BP_Character_C|GetHeldFlag _array_element)
              (:Is%20Valid
                (Development|PrintString "Can't Score"))
              (:Is%20Not%20Valid
                (Development|PrintString "Score + 1")
                (Default|ReturnFlag _heldflag)
                (Default|EnableFlag _heldflag true)
                (Default|SetFlag Player)
                (bind _asctf_game_state (Utilities|Casting|CastToCTF_GameState (Game|GetGameState)))
                (if (Variables|/Game/GameFramework/CTF_PlayerState.CTF_PlayerState_C|GetIsTeamA _asctf_player_state)
                  (Math|Integer|IncrementInt (Variables|/Game/GameFramework/CTF_GameState.CTF_GameState_C|GetTeamAScore _asctf_game_state))
                  (else
                    (Math|Integer|IncrementInt (Variables|/Game/GameFramework/CTF_GameState.CTF_GameState_C|GetTeamBScore _asctf_game_state))))))))))
    (else
      (Development|PrintString "Enemy Base"))))

(event EventBeginPlay)

(event EventTick
  (params (DeltaSeconds :type Float%20%28single-precision%29)))

(fn ConstructionScript)