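; Lobby game mode that holds an online session until a second player joins, then moves to gameplay.
; On PostLogin, a lone player starts a three-minute timeout, while any other player count triggers a server travel to the gameplay map.
; When the timer fires without exactly two players present, it destroys the session and, on success, opens the main menu.
; Print strings trace each branch.
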(event Custom|Termiante%20Session%20Check
  (bind _returnvalue (Class|GameModeBase|GetNumPlayers))
  (if (== _returnvalue 2)
    (Development|PrintString "Two players, do nothing")
    (else
      (Development|PrintString "Time to terminate")
      (|DestroySession (Game|GetPlayerController 0)
        (:OnSuccess
          (Development|PrintString "Ended session sucesfully")
          (Game|OpenLevel(byName) "MainMenu" false))
        (:OnFailure
          (Development|PrintString "Failed to end session"))))))

(event EventBeginPlay)

(event EventTick
  (params (DeltaSeconds :type Float%20%28single-precision%29)))

(event EventPostLogin
  (params (NewPlayer :type Player%20Controller%20Object%20Reference))
  (bind _returnvalue (Class|GameModeBase|GetNumPlayers))
  (if (== _returnvalue 1)
    (Development|PrintString "Starting timer")
    (Utilities|Time|SetTimerbyEvent (delegate Custom|Termiante%20Session%20Check) 1.8e+02)
    (else
      (Development|PrintString "Starting to travel")
      (Development|ExecuteConsoleCommand "servertravel gameplay" 0))))

(fn ConstructionScript)